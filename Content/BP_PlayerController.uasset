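; Player controller for a voxel world that lets the player remove blocks with the left mouse button.
; A Raycast helper line-traces along the camera view up to BlockDistance on the Visibility channel, with debug drawing.
; On a GreedyChunk hit, the impact point is nudged inward along the surface normal, converted to a local block position, and set to Air through ModifyVoxel.
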(event `Key|LeftMouseButton`
  (params (Key :type "Key Structure"))
  (:`Pressed`
    (bind (_returnvalue _outhit) (`self.Raycast`))
    (if _returnvalue
      (bind (_bblockinghit _binitialoverlap _time _distance _location _impactpoint _normal _impactnormal _physmat _hitactor) (`GameplayStatics.BreakHitResult` _outhit))
      (bind _asgreedy_chunk (cast `GreedyChunk` _hitactor))
      (`GreedyChunk.ModifyVoxel` _asgreedy_chunk (`VoxelFunctionLibrary.WorldToLocalBlockPosition` (- _location _normal) (`self.ChunkSize`)) "Air"))))

(fn `Raycast`
  (returns (ReturnValue :type Boolean) (OutHit :type "HitResult Structure"))
  (bind _playercameramanager (`self.PlayerCameraManager`))
  (bind _returnvalue (`PlayerCameraManager.GetCameraLocation` _playercameramanager))
  (bind (_outhit _returnvalue_2) (`KismetSystemLibrary.LineTraceSingle` :`Start` _returnvalue :`End` (+ _returnvalue (* (`KismetMathLibrary.GetForwardVector` (`PlayerCameraManager.GetCameraRotation` _playercameramanager)) (`self.BlockDistance`))) :`TraceChannel` "TraceTypeQuery1" :`DrawDebugType` "ForDuration" :`DrawTime` 10.0))
  (return _returnvalue_2 _outhit))

(fn `UserConstructionScript`)