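; BP_Character is a player-controlled Character Blueprint that handles basic movement and look input.
; The Horizontal and Vertical axes scale the actor's right and forward vectors and feed them to CharacterMovement as input vectors.
; The two Look axes drive controller yaw and pitch directly, and the construction script is empty.
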(event `InputAxis|Horizontal`
  (params (AxisValue :type "Float (single-precision)"))
  ;[0.1267 0.1267 0.1267] Movement
  (`PawnMovementComponent.AddInputVector` (`self.CharacterMovement`) (* AxisValue (`self.GetActorRightVector`)) false))

(event `InputAxis|Look RIght`
  (params (AxisValue :type "Float (single-precision)"))
  ;[0.1267 0.1267 0.1267] Camera
  (`self.AddControllerYawInput` AxisValue))

(event `InputAxis|Look Up`
  (params (AxisValue :type "Float (single-precision)"))
  ;[0.1267 0.1267 0.1267] Camera
  (`self.AddControllerPitchInput` AxisValue))

(event `InputAxis|Vertical`
  (params (AxisValue :type "Float (single-precision)"))
  ;[0.1267 0.1267 0.1267] Movement
  (`PawnMovementComponent.AddInputVector` (`self.CharacterMovement`) (* AxisValue (`self.GetActorForwardVector`)) false))

(fn `UserConstructionScript`)